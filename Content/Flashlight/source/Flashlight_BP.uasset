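; Flashlight actor that switches its spotlight and the glow of its mesh material on and off.
; BeginPlay binds Toggle_Event to Toggle, and each call flips the Onoff flag, setting the SpotLight intensity and the Emission material parameter together.
; The construction script applies the same settings from Onoff, so the starting state is set at construction.
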(event `self.ReceiveBeginPlay`
  (add `self.Toggle` (delegate `Toggle_Event`)))

(event `Toggle_Event`
  (bind _spotlight (`self.SpotLight`))
  (bind _flashlight (`self.Flashlight`))
  (if (`self.on/off`)
    (set `self.on/off` false)
    (`LightComponent.SetIntensity` _spotlight 0.0)
    (`MeshComponent.SetScalarParameterValueOnMaterials` _flashlight "Emission" 0.0)
    (else
      (set `self.on/off` true)
      (`LightComponent.SetIntensity` _spotlight 0.2)
      (`MeshComponent.SetScalarParameterValueOnMaterials` _flashlight "Emission" 250.0))))

(fn `UserConstructionScript`
  (bind _spotlight (`self.SpotLight`))
  (bind _flashlight (`self.Flashlight`))
  (if (`self.on/off`)
    (`LightComponent.SetIntensity` _spotlight 0.2)
    (`MeshComponent.SetScalarParameterValueOnMaterials` _flashlight "Emission" 250.0)
    (else
      (`LightComponent.SetIntensity` _spotlight 0.0)
      (`MeshComponent.SetScalarParameterValueOnMaterials` _flashlight "Emission" 0.0))))